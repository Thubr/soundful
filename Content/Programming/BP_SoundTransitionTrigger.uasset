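; BP_SoundTransitionTrigger is an overlap trigger that flips the game's audio scene and level between Woods and House.
; On BeginPlay it starts 2D FMOD transition events for music and ambience and stores both instances.
; When the player character overlaps, it reads the music instance's parameter value, toggles the global "Scene" parameter between 0 and 1, and passes the matching name to SoundfulGamemode's ChangeLevel.
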(event `self.ReceiveBeginPlay`
  (bind _returnvalue (`FMODBlueprintStatics.PlayEvent2D` "/Game/FMOD/Events/S_BGM_Transition.S_BGM_Transition"))
  (set `self.BGM` _returnvalue)
  (bind _returnvalue_2 (`FMODBlueprintStatics.PlayEvent2D` "/Game/FMOD/Events/S_Amb_Transition_2.S_Amb_Transition_2"))
  (set `self.Ambience` _returnvalue_2))

(event `self.ReceiveActorBeginOverlap`
  (params (OtherActor :type "Actor Object Reference"))
  (if (== OtherActor (`GameplayStatics.GetPlayerCharacter` 0))
    (bind _uservalue (`FMODBlueprintStatics.EventInstanceGetParameterValue` (`self.BGM`) "Scene"))
    (bind _returnvalue (< _uservalue 1.0))
    (`FMODBlueprintStatics.SetGlobalParameterByName` "Scene" (`KismetMathLibrary.SelectFloat` 1.0 0.0 _returnvalue))
    (`/Game/Programming/SoundfulGamemode.ChangeLevel` (cast `/Game/Programming/SoundfulGamemode` (`GameplayStatics.GetGameMode`) :!pure true) (select `bool` _returnvalue :`false` "House" :`true` "Woods" :!type "Name"))))

(fn `UserConstructionScript`)